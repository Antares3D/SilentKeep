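; BP_CreditsRoll is a trigger that runs the end-of-game cinematic walk and outro when the player character enters its box.
; On first overlap it disables input, turns the character toward EndWalkTarget and plays a jog animation.
; The CinematicWalk timeline pushes the character toward the target with unswept world offsets.
; When it finishes, it lowers music through a sound mix, fades in WBP_Outro and switches to UI-only input with the cursor shown.
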(event OnComponentBeginOverlap(EndCinematicTriggerBox)
  (params (OverlappedComponent :type Primitive%20Component%20Object%20Reference) (OtherActor :type Actor%20Object%20Reference) (OtherComp :type Primitive%20Component%20Object%20Reference) (OtherBodyIndex :type Integer) (bFromSweep :type Boolean) (SweepResult :type Hit%20Result%20Structure%20%28by%20ref%29))
  (bind _returnvalue (Game|GetPlayerController 0))
  (bind _endwalktarget (Variables|Default|GetEndWalkTarget))
  (bind _returnvalue_2 (Transformation|GetActorLocation _endwalktarget))
  (bind _asbp_player_character (Utilities|Casting|CastToBP_PlayerCharacter OtherActor))
  (Utilities|FlowControl|DoOnce false
    (:Completed
      (Input|DisableInput _asbp_player_character (Game|GetPlayerController 0))
      (Transformation|SetActorRotation _asbp_player_character (Math|Rotator|FindLookatRotation (Transformation|GetActorLocation _asbp_player_character) _returnvalue_2))
      (Components|Animation|PlayAnimation (Variables|/Script/Engine.Character|GetMesh _asbp_player_character) "/Game/Characters/Animations/NewMF_Unarmed_Jog_Fwd.NewMF_Unarmed_Jog_Fwd" false)
      (bind _forwardpush (Timeline|CinematicWalk PlayFromStart)
        (:Update
          (Transformation|AddActorWorldOffset _asbp_player_character (* _forwardpush (Math|Vector|GetUnitDirection(Vector) (Transformation|GetActorLocation _asbp_player_character) _returnvalue_2))))
        (:Finished
          (Audio|PushSoundMixModifier "/Game/Audio/SM_LowerMusic.SM_LowerMusic")
          (bind _returnvalue_3 (UserInterface|CreateWidget "/Game/UI/WBP_Outro.WBP_Outro_C"))
          (UserInterface|Viewport|AddtoViewport _returnvalue_3 0)
          (UserInterface|Animation|PlayAnimation _returnvalue_3 (Variables|/Game/UI/WBP_Outro.WBP_Outro_C|GetOutroFade _returnvalue_3) 0.0 1 "Forward" 1.0 false)
          (Variables|/Script/Engine.PlayerController|SetbShowMouseCursor _returnvalue true)
          (Input|SetInputModeUIOnly _returnvalue 0 "DoNotLock" false))))))

(fn ConstructionScript)