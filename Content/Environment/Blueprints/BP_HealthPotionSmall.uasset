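; BP_HealthPotionSmall is an interactable small health potion that restores a little of the player's HP when drunk.
; Overlapping its interaction box registers it as the player's current interactable and shows a prompt on the main UI, and leaving clears both.
; Interact adds a fixed amount to player zero's HP within a clamped range, plays a bottle sound and destroys the potion.
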(event OnComponentBeginOverlap(InteractionBox)
  (params (OverlappedComponent :type Primitive%20Component%20Object%20Reference) (OtherActor :type Actor%20Object%20Reference) (OtherComp :type Primitive%20Component%20Object%20Reference) (OtherBodyIndex :type Integer) (bFromSweep :type Boolean) (SweepResult :type Hit%20Result%20Structure%20%28by%20ref%29))
  (bind _asbp_player_character (Utilities|Casting|CastToBP_PlayerCharacter OtherActor))
  (Default|SetCurrentInteractable _asbp_player_character self)
  (Rendering|Components|TextRender|SetText (Variables|/Game/UI/WBP_MainInterface.WBP_MainInterface_C|GetInteractionText (Variables|/Game/Characters/Player/Blueprints/BP_PlayerCharacter.BP_PlayerCharacter_C|GetMainUI _asbp_player_character)) "PRESS E TO DRINK HEALTH POTION (SMALL)")
  (Widget|SetVisibility (Variables|/Game/UI/WBP_MainInterface.WBP_MainInterface_C|GetInteractionText (Variables|/Game/Characters/Player/Blueprints/BP_PlayerCharacter.BP_PlayerCharacter_C|GetMainUI _asbp_player_character)) "Visible"))

(event OnComponentEndOverlap(InteractionBox)
  (params (OverlappedComponent :type Primitive%20Component%20Object%20Reference) (OtherActor :type Actor%20Object%20Reference) (OtherComp :type Primitive%20Component%20Object%20Reference) (OtherBodyIndex :type Integer))
  (bind _asbp_player_character (Utilities|Casting|CastToBP_PlayerCharacter OtherActor))
  (Default|SetCurrentInteractable _asbp_player_character)
  (Widget|SetVisibility (Variables|/Game/UI/WBP_MainInterface.WBP_MainInterface_C|GetInteractionText (Variables|/Game/Characters/Player/Blueprints/BP_PlayerCharacter.BP_PlayerCharacter_C|GetMainUI _asbp_player_character)) "Hidden"))

(event EventInteract
  (bind _asbp_player_character (Utilities|Casting|CastToBP_PlayerCharacter (Game|GetPlayerCharacter 0)))
  (Variables|/Game/Characters/Player/Blueprints/BP_PlayerCharacter.BP_PlayerCharacter_C|SetCurrentHP _asbp_player_character (Math|Float|Clamp(Float) (+ (Variables|/Game/Characters/Player/Blueprints/BP_PlayerCharacter.BP_PlayerCharacter_C|GetCurrentHP _asbp_player_character) 1e+01) 0.0 1e+02))
  (Audio|PlaySound2D "/Game/Audio/Effects/Bottle.Bottle" 1.0 1.0 0.0 0 0)
  (Actor|DestroyActor))

(fn ConstructionScript)