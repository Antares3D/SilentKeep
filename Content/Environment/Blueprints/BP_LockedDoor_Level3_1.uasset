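; Locked door that the player opens with the training room key, then toggles open and closed through Interact.
; An overlap box registers it as the player's current interactable and shows a lock-aware UI prompt.
; A Timeline swings the pivot in yaw, played or reversed, with IsInteracting blocking re-entry until it finishes.
; UnlockDoor clears the lock directly; the prompt set during a toggle reflects the state before the swing.
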(event OnComponentBeginOverlap(InteractionBox)
  (params (OverlappedComponent :type Primitive%20Component%20Object%20Reference) (OtherActor :type Actor%20Object%20Reference) (OtherComp :type Primitive%20Component%20Object%20Reference) (OtherBodyIndex :type Integer) (bFromSweep :type Boolean) (SweepResult :type Hit%20Result%20Structure%20%28by%20ref%29))
  (bind _returnvalue (Game|GetPlayerCharacter 0))
  (bind _asbp_player_character (Utilities|Casting|CastToBP_PlayerCharacter OtherActor))
  (Default|SetCurrentInteractable _asbp_player_character self)
  (Widget|SetVisibility (Variables|/Game/UI/WBP_MainInterface.WBP_MainInterface_C|GetInteractionText (Variables|/Game/Characters/Player/Blueprints/BP_PlayerCharacter.BP_PlayerCharacter_C|GetMainUI _asbp_player_character)) "Visible")
  (if (Variables|Default|GetIsLocked)
    (bind _asbp_player_character_2 (Utilities|Casting|CastToBP_PlayerCharacter _returnvalue))
    (if (Variables|/Game/Characters/Player/Blueprints/BP_PlayerCharacter.BP_PlayerCharacter_C|GetHasTrainingRoomKey _asbp_player_character_2)
      (Rendering|Components|TextRender|SetText (Variables|/Game/UI/WBP_MainInterface.WBP_MainInterface_C|GetInteractionText (Variables|/Game/Characters/Player/Blueprints/BP_PlayerCharacter.BP_PlayerCharacter_C|GetMainUI _asbp_player_character_2)) "PRESS E TO OPEN")
      (else
        (Rendering|Components|TextRender|SetText (Variables|/Game/UI/WBP_MainInterface.WBP_MainInterface_C|GetInteractionText (Variables|/Game/Characters/Player/Blueprints/BP_PlayerCharacter.BP_PlayerCharacter_C|GetMainUI _asbp_player_character_2)) "DOOR LOCKED. KEY REQUIRED!")))
    (elif (Variables|Default|GetIsOpen)
      (bind _asbp_player_character_3 (Utilities|Casting|CastToBP_PlayerCharacter _returnvalue))
      (Rendering|Components|TextRender|SetText (Variables|/Game/UI/WBP_MainInterface.WBP_MainInterface_C|GetInteractionText (Variables|/Game/Characters/Player/Blueprints/BP_PlayerCharacter.BP_PlayerCharacter_C|GetMainUI _asbp_player_character_3)) "PRESS E TO CLOSE")
      (else
        (bind _asbp_player_character_4 (Utilities|Casting|CastToBP_PlayerCharacter _returnvalue))
        (Rendering|Components|TextRender|SetText (Variables|/Game/UI/WBP_MainInterface.WBP_MainInterface_C|GetInteractionText (Variables|/Game/Characters/Player/Blueprints/BP_PlayerCharacter.BP_PlayerCharacter_C|GetMainUI _asbp_player_character_4)) "PRESS E TO OPEN")))))

(event OnComponentEndOverlap(InteractionBox)
  (params (OverlappedComponent :type Primitive%20Component%20Object%20Reference) (OtherActor :type Actor%20Object%20Reference) (OtherComp :type Primitive%20Component%20Object%20Reference) (OtherBodyIndex :type Integer))
  (bind _asbp_player_character (Utilities|Casting|CastToBP_PlayerCharacter OtherActor))
  (Default|SetCurrentInteractable _asbp_player_character)
  (Widget|SetVisibility (Variables|/Game/UI/WBP_MainInterface.WBP_MainInterface_C|GetInteractionText (Variables|/Game/Characters/Player/Blueprints/BP_PlayerCharacter.BP_PlayerCharacter_C|GetMainUI _asbp_player_character)) "Hidden"))

(event EventInteract
  (bind _returnvalue (Game|GetPlayerCharacter 0))
  (if (Variables|Default|GetIsLocked)
    (bind _asbp_player_character (Utilities|Casting|CastToBP_PlayerCharacter (Game|GetPlayerCharacter 0)))
    (if (Variables|/Game/Characters/Player/Blueprints/BP_PlayerCharacter.BP_PlayerCharacter_C|GetHasTrainingRoomKey _asbp_player_character)
      (Variables|Default|SetIsLocked false)
      (if (not (Variables|Default|GetbIsInteracting)) :!label _label
        (Variables|Default|SetbIsInteracting true)
        (if (Variables|Default|GetIsOpen)
          (Audio|PlaySound2D "/Game/Audio/Effects/Door_Open_2.Door_Open_2" 1.0 1.0 0.0 0 0)
          (bind _asbp_player_character_2 (Utilities|Casting|CastToBP_PlayerCharacter _returnvalue))
          (Rendering|Components|TextRender|SetText (Variables|/Game/UI/WBP_MainInterface.WBP_MainInterface_C|GetInteractionText (Variables|/Game/Characters/Player/Blueprints/BP_PlayerCharacter.BP_PlayerCharacter_C|GetMainUI _asbp_player_character_2)) "PRESS E TO CLOSE")
          (bind _tl_opendoor (Timeline|Timeline Reverse)
            (:Update
              (Transformation|SetRelativeRotation (Variables|Default|GetPivotDoor) (Math|Rotator|MakeRotator 0.0 0.0 (* _tl_opendoor -9e+01)) false false))
            (:Finished
              (Variables|Default|SetIsOpen (not (Variables|Default|GetIsOpen)))
              (Variables|Default|SetbIsInteracting false)))
          (else
            (Audio|PlaySound2D "/Game/Audio/Effects/Door_Open_2.Door_Open_2" 1.0 1.0 0.0 0 0)
            (bind _asbp_player_character_3 (Utilities|Casting|CastToBP_PlayerCharacter _returnvalue))
            (Rendering|Components|TextRender|SetText (Variables|/Game/UI/WBP_MainInterface.WBP_MainInterface_C|GetInteractionText (Variables|/Game/Characters/Player/Blueprints/BP_PlayerCharacter.BP_PlayerCharacter_C|GetMainUI _asbp_player_character_3)) "PRESS E TO OPEN")
            (Timeline|Timeline Play))))
      (else
        (Rendering|Components|TextRender|SetText (Variables|/Game/UI/WBP_MainInterface.WBP_MainInterface_C|GetInteractionText (Variables|/Game/Characters/Player/Blueprints/BP_PlayerCharacter.BP_PlayerCharacter_C|GetMainUI _asbp_player_character)) "DOOR LOCKED. KEY REQUIRED!")
        (Audio|PlaySound2D "/Game/Audio/Effects/Locked_Door.Locked_Door" 1.0 1.0 0.0 0 0)))
    (else
      (goto _label))))

(fn ConstructionScript)

(fn UnlockDoor
  (Variables|Default|SetIsLocked false))