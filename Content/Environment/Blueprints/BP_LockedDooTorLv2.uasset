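; BP_LockedDooTorLv2 is a key-locked door that sends the player to LV_Level_2.
; Overlapping its InteractionBox registers it as the player's current interactable and shows a prompt in MainUI, which reflects HasKey while locked.
; Interact with the key unlocks it, plays a sound and screen fade, then opens the level after a delay; without, it shows a locked warning.
; UnlockDoor only clears IsLocked, and Interact ignores unlocked doors.
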(event OnComponentBeginOverlap(InteractionBox)
  (params (OverlappedComponent :type Primitive%20Component%20Object%20Reference) (OtherActor :type Actor%20Object%20Reference) (OtherComp :type Primitive%20Component%20Object%20Reference) (OtherBodyIndex :type Integer) (bFromSweep :type Boolean) (SweepResult :type Hit%20Result%20Structure%20%28by%20ref%29))
  (bind _asbp_player_character (Utilities|Casting|CastToBP_PlayerCharacter OtherActor))
  (Default|SetCurrentInteractable _asbp_player_character self)
  (Widget|SetVisibility (Variables|/Game/UI/WBP_MainInterface.WBP_MainInterface_C|GetInteractionText (Variables|/Game/Characters/Player/Blueprints/BP_PlayerCharacter.BP_PlayerCharacter_C|GetMainUI _asbp_player_character)) "Visible")
  (if (Variables|Default|GetIsLocked)
    (bind _asbp_player_character_2 (Utilities|Casting|CastToBP_PlayerCharacter (Game|GetPlayerCharacter 0)))
    (if (Variables|/Game/Characters/Player/Blueprints/BP_PlayerCharacter.BP_PlayerCharacter_C|GetHasKey _asbp_player_character_2)
      (Rendering|Components|TextRender|SetText (Variables|/Game/UI/WBP_MainInterface.WBP_MainInterface_C|GetInteractionText (Variables|/Game/Characters/Player/Blueprints/BP_PlayerCharacter.BP_PlayerCharacter_C|GetMainUI _asbp_player_character_2)) "PRESS E TO OPEN")
      (else
        (Rendering|Components|TextRender|SetText (Variables|/Game/UI/WBP_MainInterface.WBP_MainInterface_C|GetInteractionText (Variables|/Game/Characters/Player/Blueprints/BP_PlayerCharacter.BP_PlayerCharacter_C|GetMainUI _asbp_player_character_2)) "DOOR LOCKED. KEY REQUIRED!")))))

(event OnComponentEndOverlap(InteractionBox)
  (params (OverlappedComponent :type Primitive%20Component%20Object%20Reference) (OtherActor :type Actor%20Object%20Reference) (OtherComp :type Primitive%20Component%20Object%20Reference) (OtherBodyIndex :type Integer))
  (bind _asbp_player_character (Utilities|Casting|CastToBP_PlayerCharacter OtherActor))
  (Default|SetCurrentInteractable _asbp_player_character)
  (Widget|SetVisibility (Variables|/Game/UI/WBP_MainInterface.WBP_MainInterface_C|GetInteractionText (Variables|/Game/Characters/Player/Blueprints/BP_PlayerCharacter.BP_PlayerCharacter_C|GetMainUI _asbp_player_character)) "Hidden"))

(event EventInteract
  (if (Variables|Default|GetIsLocked)
    (bind _asbp_player_character (Utilities|Casting|CastToBP_PlayerCharacter (Game|GetPlayerCharacter 0)))
    (if (Variables|/Game/Characters/Player/Blueprints/BP_PlayerCharacter.BP_PlayerCharacter_C|GetHasKey _asbp_player_character)
      (Variables|Default|SetIsLocked false)
      (Audio|PlaySound2D "/Game/Audio/Effects/Door_Open_2.Door_Open_2" 1.0 1.0 0.0 0 0)
      (bind _asbp_player_character_2 (Utilities|Casting|CastToBP_PlayerCharacter (Game|GetPlayerCharacter 0)))
      (Rendering|Components|TextRender|SetText (Variables|/Game/UI/WBP_MainInterface.WBP_MainInterface_C|GetInteractionText (Variables|/Game/Characters/Player/Blueprints/BP_PlayerCharacter.BP_PlayerCharacter_C|GetMainUI _asbp_player_character_2)) "PRESS E TO OPEN")
      (Widget|SetVisibility (Variables|/Game/UI/WBP_MainInterface.WBP_MainInterface_C|GetFadeScreen (Variables|/Game/Characters/Player/Blueprints/BP_PlayerCharacter.BP_PlayerCharacter_C|GetMainUI _asbp_player_character_2)) "Visible")
      (UserInterface|Animation|PlayAnimation (Variables|/Game/Characters/Player/Blueprints/BP_PlayerCharacter.BP_PlayerCharacter_C|GetMainUI _asbp_player_character_2) (Variables|/Game/UI/WBP_MainInterface.WBP_MainInterface_C|GetInterfaceFade (Variables|/Game/Characters/Player/Blueprints/BP_PlayerCharacter.BP_PlayerCharacter_C|GetMainUI _asbp_player_character_2)) 0.0 1 "Forward" 1.0 false)
      (Utilities|FlowControl|Delay 1.0)
      (Game|OpenLevel(byObjectReference) "/Game/Levels/LV_Level_2.LV_Level_2")
      (else
        (Rendering|Components|TextRender|SetText (Variables|/Game/UI/WBP_MainInterface.WBP_MainInterface_C|GetInteractionText (Variables|/Game/Characters/Player/Blueprints/BP_PlayerCharacter.BP_PlayerCharacter_C|GetMainUI _asbp_player_character)) "DOOR LOCKED. KEY REQUIRED!")
        (Audio|PlaySound2D "/Game/Audio/Effects/Locked_Door.Locked_Door" 1.0 1.0 0.0 0 0)))))

(fn ConstructionScript)

(fn UnlockDoor
  (Variables|Default|SetIsLocked false))