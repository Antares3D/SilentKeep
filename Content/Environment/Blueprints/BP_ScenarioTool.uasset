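; BP_ScenarioTool is a construction-script tool that fills an area with a flat grid of instanced static meshes.
; It divides DrawVector's X and Y by Size, truncates the results, and adds an instance at each grid point spaced Size apart.
; Both loops include their end index, so each axis gets one more instance than the truncated count.
; The event graph holds only disabled stub events.
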(event EventBeginPlay)

(event Collision|EventActorBeginOverlap
  (params (OtherActor :type Actor%20Object%20Reference)))

(event EventTick
  (params (DeltaSeconds :type Float%20%28single-precision%29)))

(fn ConstructionScript
  (bind _drawvector (Variables|Default|GetDrawVector))
  (bind _size (Variables|Default|GetSize))
  (bind _size_2 (Variables|Default|GetSize))
  (LocalVariables|Setx (Math|Float|Truncate (/ (.x _drawvector) _size)))
  (LocalVariables|SetY (Math|Float|Truncate (/ (.y _drawvector) _size)))
  (for _index (range 0 (LocalVariables|Getx))
    (for _index_2 (range 0 (LocalVariables|GetY))
      (Components|InstancedStaticMesh|AddInstance (Variables|Default|GetInstancedStaticMesh) (Math|Transform|MakeTransform (Math|Vector|MakeVector (* _index _size_2) (* _index_2 _size_2) 0.0) "0, 0, 0" "1.000000,1.000000,1.000000") false))))