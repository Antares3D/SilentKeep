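; BP_LockedGate_LV3 is an interactable gate that stays locked until the player has the prison key.
; An interaction box registers it as the player's current interactable and shows a state-based prompt in the main UI.
; Interact unlocks it with the key, then plays or reverses a timeline that slides the Pivot vertically with a chain sound.
; Without the key it shows a locked message; UnlockDoor can also clear the lock directly.
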(event OnComponentBeginOverlap(InteractionBox)
  (params (OverlappedComponent :type Primitive%20Component%20Object%20Reference) (OtherActor :type Actor%20Object%20Reference) (OtherComp :type Primitive%20Component%20Object%20Reference) (OtherBodyIndex :type Integer) (bFromSweep :type Boolean) (SweepResult :type Hit%20Result%20Structure%20%28by%20ref%29))
  (bind _returnvalue (Game|GetPlayerCharacter 0))
  (bind _asbp_player_character (Utilities|Casting|CastToBP_PlayerCharacter OtherActor))
  (Default|SetCurrentInteractable _asbp_player_character self)
  (Widget|SetVisibility (Variables|/Game/UI/WBP_MainInterface.WBP_MainInterface_C|GetInteractionText (Variables|/Game/Characters/Player/Blueprints/BP_PlayerCharacter.BP_PlayerCharacter_C|GetMainUI _asbp_player_character)) "Visible")
  (if (Variables|Default|GetIsLocked)
    (bind _asbp_player_character_2 (Utilities|Casting|CastToBP_PlayerCharacter _returnvalue))
    (if (Variables|/Game/Characters/Player/Blueprints/BP_PlayerCharacter.BP_PlayerCharacter_C|GetHasPrisonKey _asbp_player_character_2)
      (Rendering|Components|TextRender|SetText (Variables|/Game/UI/WBP_MainInterface.WBP_MainInterface_C|GetInteractionText (Variables|/Game/Characters/Player/Blueprints/BP_PlayerCharacter.BP_PlayerCharacter_C|GetMainUI _asbp_player_character_2)) "PRESS E TO OPEN")
      (else
        (Rendering|Components|TextRender|SetText (Variables|/Game/UI/WBP_MainInterface.WBP_MainInterface_C|GetInteractionText (Variables|/Game/Characters/Player/Blueprints/BP_PlayerCharacter.BP_PlayerCharacter_C|GetMainUI _asbp_player_character_2)) "GATE LOCKED!")))
    (elif (Variables|Default|GetIsOpen)
      (bind _asbp_player_character_3 (Utilities|Casting|CastToBP_PlayerCharacter _returnvalue))
      (Rendering|Components|TextRender|SetText (Variables|/Game/UI/WBP_MainInterface.WBP_MainInterface_C|GetInteractionText (Variables|/Game/Characters/Player/Blueprints/BP_PlayerCharacter.BP_PlayerCharacter_C|GetMainUI _asbp_player_character_3)) "PRESS E TO CLOSE")
      (else
        (bind _asbp_player_character_4 (Utilities|Casting|CastToBP_PlayerCharacter _returnvalue))
        (Rendering|Components|TextRender|SetText (Variables|/Game/UI/WBP_MainInterface.WBP_MainInterface_C|GetInteractionText (Variables|/Game/Characters/Player/Blueprints/BP_PlayerCharacter.BP_PlayerCharacter_C|GetMainUI _asbp_player_character_4)) "PRESS E TO OPEN")))))

(event OnComponentEndOverlap(InteractionBox)
  (params (OverlappedComponent :type Primitive%20Component%20Object%20Reference) (OtherActor :type Actor%20Object%20Reference) (OtherComp :type Primitive%20Component%20Object%20Reference) (OtherBodyIndex :type Integer))
  (bind _asbp_player_character (Utilities|Casting|CastToBP_PlayerCharacter OtherActor))
  (Default|SetCurrentInteractable _asbp_player_character)
  (Widget|SetVisibility (Variables|/Game/UI/WBP_MainInterface.WBP_MainInterface_C|GetInteractionText (Variables|/Game/Characters/Player/Blueprints/BP_PlayerCharacter.BP_PlayerCharacter_C|GetMainUI _asbp_player_character)) "Hidden"))

(event EventBeginPlay
  (Variables|Default|SetInitialLocation (Variables|/Script/Engine.SceneComponent|GetRelativeLocation (Variables|Default|GetPivot))))

(event EventInteract
  (bind _returnvalue (Game|GetPlayerCharacter 0))
  (if (Variables|Default|GetIsLocked)
    (bind _asbp_player_character (Utilities|Casting|CastToBP_PlayerCharacter (Game|GetPlayerCharacter 0)))
    (if (Variables|/Game/Characters/Player/Blueprints/BP_PlayerCharacter.BP_PlayerCharacter_C|GetHasPrisonKey _asbp_player_character)
      (Variables|Default|SetIsLocked false)
      (if (Variables|Default|GetIsOpen) :!label _label
        (Audio|PlaySound2D "/Game/Audio/Effects/Chain.Chain" 1.0 1.0 0.0 0 0)
        (bind _asbp_player_character_2 (Utilities|Casting|CastToBP_PlayerCharacter _returnvalue))
        (Rendering|Components|TextRender|SetText (Variables|/Game/UI/WBP_MainInterface.WBP_MainInterface_C|GetInteractionText (Variables|/Game/Characters/Player/Blueprints/BP_PlayerCharacter.BP_PlayerCharacter_C|GetMainUI _asbp_player_character_2)) "PRESS E TO CLOSE")
        (bind _tl_opendoor (Timeline|Timeline_0 Reverse)
          (:Update
            (Transformation|SetRelativeLocation (Variables|Default|GetPivot) (+ (Variables|Default|GetInitialLocation) (Math|Vector|MakeVector 0.0 0.0 (* _tl_opendoor 3.5e+02))) false false))
          (:Finished
            (Variables|Default|SetIsOpen (not (Variables|Default|GetIsOpen)))))
        (else
          (Audio|PlaySound2D "/Game/Audio/Effects/Chain.Chain" 1.0 1.0 0.0 0 0)
          (bind _asbp_player_character_3 (Utilities|Casting|CastToBP_PlayerCharacter _returnvalue))
          (Rendering|Components|TextRender|SetText (Variables|/Game/UI/WBP_MainInterface.WBP_MainInterface_C|GetInteractionText (Variables|/Game/Characters/Player/Blueprints/BP_PlayerCharacter.BP_PlayerCharacter_C|GetMainUI _asbp_player_character_3)) "PRESS E TO OPEN")
          (Timeline|Timeline_0 Play)))
      (else
        (Rendering|Components|TextRender|SetText (Variables|/Game/UI/WBP_MainInterface.WBP_MainInterface_C|GetInteractionText (Variables|/Game/Characters/Player/Blueprints/BP_PlayerCharacter.BP_PlayerCharacter_C|GetMainUI _asbp_player_character)) "GATE LOCKED!")
        (Audio|PlaySound2D "/Game/Audio/Effects/Metal_1.Metal_1" 1.0 1.0 0.0 0 0)))
    (else
      (goto _label))))

(fn ConstructionScript)

(fn UnlockDoor
  (Variables|Default|SetIsLocked false))