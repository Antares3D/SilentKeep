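; BP_QuestTrigger is a one-shot quest trigger volume that shows the objective "Open the Door" on screen.
; Box overlap creates a WBP_MainInterface with that text, then sets HasTriggered only if the actor is BP_PlayerCharacter.
; End overlap removes the widget after a short delay.
; Both player casts run after the widget changes, so any overlapping actor can show or remove the prompt.
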(event OnComponentBeginOverlap(Box)
  (params (OverlappedComponent :type Primitive%20Component%20Object%20Reference) (OtherActor :type Actor%20Object%20Reference) (OtherComp :type Primitive%20Component%20Object%20Reference) (OtherBodyIndex :type Integer) (bFromSweep :type Boolean) (SweepResult :type Hit%20Result%20Structure%20%28by%20ref%29))
  ;[0.02178 0.02619 0.15 0.5 12] Has the Quest been triggered?
  (if (not (Variables|Default|GetHasTriggered))
    (Variables|Default|SetPromptText (Utilities|Text|MakeLiteralText "Objective: 
Open the Door"))
    (bind _returnvalue (UserInterface|CreateWidget "/Game/UI/WBP_MainInterface.WBP_MainInterface_C" (Game|GetPlayerController 0) (Variables|Default|GetPromptText)))
    (bind _output_get (Variables|Default|SetInteractionPrompt _returnvalue))
    (UserInterface|Viewport|AddtoViewport _output_get 0)
    (Utilities|Casting|CastToBP_PlayerCharacter OtherActor)
    (Variables|Default|SetHasTriggered true)))

(event OnComponentEndOverlap(Box)
  (params (OverlappedComponent :type Primitive%20Component%20Object%20Reference) (OtherActor :type Actor%20Object%20Reference) (OtherComp :type Primitive%20Component%20Object%20Reference) (OtherBodyIndex :type Integer))
  (Utilities|FlowControl|Delay 2.0)
  (Utilities|IsValid (Variables|Default|GetInteractionPrompt)
    (:Is%20Valid
      (Widget|RemovefromParent (Variables|Default|GetInteractionPrompt))
      (Variables|Default|SetInteractionPrompt 0)
      (Utilities|Casting|CastToBP_PlayerCharacter OtherActor))))

(fn ConstructionScript)