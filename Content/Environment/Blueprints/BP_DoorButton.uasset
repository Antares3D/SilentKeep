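; Interactable wall or floor button that, when pressed, destroys its linked spikes and unlocks a referenced door.
; An overlap box registers it as the player's current interactable and shows a prompt or activated message in the main UI.
; Interacting plays a grinding sound and fires a one-shot timeline that slides the pivot in, then reverses it.
; Activation and door unlock happen inside the spike loop, so both require a valid spike.
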(event OnComponentBeginOverlap(InteractionBox)
  (params (OverlappedComponent :type Primitive%20Component%20Object%20Reference) (OtherActor :type Actor%20Object%20Reference) (OtherComp :type Primitive%20Component%20Object%20Reference) (OtherBodyIndex :type Integer) (bFromSweep :type Boolean) (SweepResult :type Hit%20Result%20Structure%20%28by%20ref%29))
  (if (Variables|Default|GetButtonActivated)
    (bind _asbp_player_character (Utilities|Casting|CastToBP_PlayerCharacter OtherActor))
    (Default|SetCurrentInteractable _asbp_player_character self)
    (Rendering|Components|TextRender|SetText (Variables|/Game/UI/WBP_MainInterface.WBP_MainInterface_C|GetInteractionText (Variables|/Game/Characters/Player/Blueprints/BP_PlayerCharacter.BP_PlayerCharacter_C|GetMainUI _asbp_player_character)) "BUTTON ACTIVATED!")
    (Widget|SetVisibility (Variables|/Game/UI/WBP_MainInterface.WBP_MainInterface_C|GetInteractionText (Variables|/Game/Characters/Player/Blueprints/BP_PlayerCharacter.BP_PlayerCharacter_C|GetMainUI _asbp_player_character)) "Visible")
    (else
      (bind _asbp_player_character_2 (Utilities|Casting|CastToBP_PlayerCharacter OtherActor))
      (Default|SetCurrentInteractable _asbp_player_character_2 self)
      (Rendering|Components|TextRender|SetText (Variables|/Game/UI/WBP_MainInterface.WBP_MainInterface_C|GetInteractionText (Variables|/Game/Characters/Player/Blueprints/BP_PlayerCharacter.BP_PlayerCharacter_C|GetMainUI _asbp_player_character_2)) "PRESS E TO ACTIVATE")
      (Widget|SetVisibility (Variables|/Game/UI/WBP_MainInterface.WBP_MainInterface_C|GetInteractionText (Variables|/Game/Characters/Player/Blueprints/BP_PlayerCharacter.BP_PlayerCharacter_C|GetMainUI _asbp_player_character_2)) "Visible"))))

(event OnComponentEndOverlap(InteractionBox)
  (params (OverlappedComponent :type Primitive%20Component%20Object%20Reference) (OtherActor :type Actor%20Object%20Reference) (OtherComp :type Primitive%20Component%20Object%20Reference) (OtherBodyIndex :type Integer))
  (bind _asbp_player_character (Utilities|Casting|CastToBP_PlayerCharacter OtherActor))
  (Default|SetCurrentInteractable _asbp_player_character)
  (Widget|SetVisibility (Variables|/Game/UI/WBP_MainInterface.WBP_MainInterface_C|GetInteractionText (Variables|/Game/Characters/Player/Blueprints/BP_PlayerCharacter.BP_PlayerCharacter_C|GetMainUI _asbp_player_character)) "Hidden"))

(event Custom|ReturnButton
  (bind _doortounlock (Variables|Default|GetDoorToUnlock))
  ;[0.004325 0 0.04167 0.5] Button Logic
  (bind _buttontimeline (Timeline|Timeline Reverse)
    (:Update
      (Transformation|SetRelativeLocation (Variables|Default|GetPivot) (+ (Variables|Default|GetInitialLocation) (Math|Vector|MakeVector 0.0 (* _buttontimeline -7.5) 0.0)) false false))
    (:Finished
      (CallFunction|ReturnButton)
      (for _array_element (Variables|Default|GetSpikesReference)
        (Utilities|IsValid _array_element
          (:Is%20Valid
            (Actor|DestroyActor (Variables|Default|GetSpikesReference))
            (Variables|Default|SetButtonActivated true)
            (Utilities|IsValid _doortounlock
              (:Is%20Valid
                (Default|UnlockDoor _doortounlock)))))))))

(event EventBeginPlay
  (Variables|Default|SetInitialLocation (Variables|/Script/Engine.SceneComponent|GetRelativeLocation (Variables|Default|GetPivot))))

(event EventInteract
  (bind _doortounlock (Variables|Default|GetDoorToUnlock))
  ;[0.004325 0 0.04167 0.5] Button Logic
  (if (Variables|Default|GetButtonActivated)
    (bind _asbp_player_character (Utilities|Casting|CastToBP_PlayerCharacter (Game|GetPlayerCharacter 0)))
    (Rendering|Components|TextRender|SetText (Variables|/Game/UI/WBP_MainInterface.WBP_MainInterface_C|GetInteractionText (Variables|/Game/Characters/Player/Blueprints/BP_PlayerCharacter.BP_PlayerCharacter_C|GetMainUI _asbp_player_character)) "BUTTON ACTIVATED!")
    (else
      (Audio|PlaySound2D "/Game/Audio/Effects/Stone_Grind.Stone_Grind" 1.0 1.0 0.0 0 0)
      (Utilities|FlowControl|DoOnce false
        (:Completed
          (bind _asbp_player_character_2 (Utilities|Casting|CastToBP_PlayerCharacter (Game|GetPlayerCharacter 0)))
          (Rendering|Components|TextRender|SetText (Variables|/Game/UI/WBP_MainInterface.WBP_MainInterface_C|GetInteractionText (Variables|/Game/Characters/Player/Blueprints/BP_PlayerCharacter.BP_PlayerCharacter_C|GetMainUI _asbp_player_character_2)) "PRESS E TO ACTIVATE")
          (bind _buttontimeline (Timeline|Timeline PlayFromStart)
            (:Update
              (Transformation|SetRelativeLocation (Variables|Default|GetPivot) (+ (Variables|Default|GetInitialLocation) (Math|Vector|MakeVector 0.0 (* _buttontimeline -7.5) 0.0)) false false))
            (:Finished
              (CallFunction|ReturnButton)
              (for _array_element (Variables|Default|GetSpikesReference)
                (Utilities|IsValid _array_element
                  (:Is%20Valid
                    (Actor|DestroyActor (Variables|Default|GetSpikesReference))
                    (Variables|Default|SetButtonActivated true)
                    (Utilities|IsValid _doortounlock
                      (:Is%20Valid
                        (Default|UnlockDoor _doortounlock)))))))))))))

(fn ConstructionScript)