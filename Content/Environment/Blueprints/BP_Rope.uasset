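; BP_Rope is an interactable escape rope that takes the player to the next level, gated on having the gemstone.
; Its InteractionBox overlap registers it as the player's current interactable and shows a prompt that depends on HasGemStone, then clears both on exit.
; Interact rechecks the gemstone, then either fades the screen and opens LV_Level_4 after a short delay or shows a refusal message.
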(event OnComponentBeginOverlap(InteractionBox)
  (params (OverlappedComponent :type Primitive%20Component%20Object%20Reference) (OtherActor :type Actor%20Object%20Reference) (OtherComp :type Primitive%20Component%20Object%20Reference) (OtherBodyIndex :type Integer) (bFromSweep :type Boolean) (SweepResult :type Hit%20Result%20Structure%20%28by%20ref%29))
  (bind _asbp_player_character (Utilities|Casting|CastToBP_PlayerCharacter OtherActor))
  (Default|SetCurrentInteractable _asbp_player_character self)
  (Widget|SetVisibility (Variables|/Game/UI/WBP_MainInterface.WBP_MainInterface_C|GetInteractionText (Variables|/Game/Characters/Player/Blueprints/BP_PlayerCharacter.BP_PlayerCharacter_C|GetMainUI _asbp_player_character)) "Visible")
  (bind _asbp_player_character_2 (Utilities|Casting|CastToBP_PlayerCharacter (Game|GetPlayerCharacter 0)))
  (if (Variables|/Game/Characters/Player/Blueprints/BP_PlayerCharacter.BP_PlayerCharacter_C|GetHasGemStone _asbp_player_character_2)
    (Rendering|Components|TextRender|SetText (Variables|/Game/UI/WBP_MainInterface.WBP_MainInterface_C|GetInteractionText (Variables|/Game/Characters/Player/Blueprints/BP_PlayerCharacter.BP_PlayerCharacter_C|GetMainUI _asbp_player_character_2)) "PRESS E TO ESCAPE")
    (else
      (Rendering|Components|TextRender|SetText (Variables|/Game/UI/WBP_MainInterface.WBP_MainInterface_C|GetInteractionText (Variables|/Game/Characters/Player/Blueprints/BP_PlayerCharacter.BP_PlayerCharacter_C|GetMainUI _asbp_player_character_2)) "YOU CAN'T LEAVE WITHOUT THE GEMSTONE!"))))

(event OnComponentEndOverlap(InteractionBox)
  (params (OverlappedComponent :type Primitive%20Component%20Object%20Reference) (OtherActor :type Actor%20Object%20Reference) (OtherComp :type Primitive%20Component%20Object%20Reference) (OtherBodyIndex :type Integer))
  (bind _asbp_player_character (Utilities|Casting|CastToBP_PlayerCharacter OtherActor))
  (Default|SetCurrentInteractable _asbp_player_character)
  (Widget|SetVisibility (Variables|/Game/UI/WBP_MainInterface.WBP_MainInterface_C|GetInteractionText (Variables|/Game/Characters/Player/Blueprints/BP_PlayerCharacter.BP_PlayerCharacter_C|GetMainUI _asbp_player_character)) "Hidden"))

(event EventInteract
  (bind _asbp_player_character (Utilities|Casting|CastToBP_PlayerCharacter (Game|GetPlayerCharacter 0)))
  (if (Variables|/Game/Characters/Player/Blueprints/BP_PlayerCharacter.BP_PlayerCharacter_C|GetHasGemStone _asbp_player_character)
    (bind _asbp_player_character_2 (Utilities|Casting|CastToBP_PlayerCharacter (Game|GetPlayerCharacter 0)))
    (Rendering|Components|TextRender|SetText (Variables|/Game/UI/WBP_MainInterface.WBP_MainInterface_C|GetInteractionText (Variables|/Game/Characters/Player/Blueprints/BP_PlayerCharacter.BP_PlayerCharacter_C|GetMainUI _asbp_player_character_2)) "PRESS E TO ESCAPE")
    (Widget|SetVisibility (Variables|/Game/UI/WBP_MainInterface.WBP_MainInterface_C|GetFadeScreen (Variables|/Game/Characters/Player/Blueprints/BP_PlayerCharacter.BP_PlayerCharacter_C|GetMainUI _asbp_player_character_2)) "Visible")
    (UserInterface|Animation|PlayAnimation (Variables|/Game/Characters/Player/Blueprints/BP_PlayerCharacter.BP_PlayerCharacter_C|GetMainUI _asbp_player_character_2) (Variables|/Game/UI/WBP_MainInterface.WBP_MainInterface_C|GetInterfaceFade (Variables|/Game/Characters/Player/Blueprints/BP_PlayerCharacter.BP_PlayerCharacter_C|GetMainUI _asbp_player_character_2)) 0.0 1 "Forward" 1.0 false)
    (Utilities|FlowControl|Delay 1.0)
    (Game|OpenLevel(byObjectReference) "/Game/Levels/LV_Level_4.LV_Level_4")
    (else
      (Rendering|Components|TextRender|SetText (Variables|/Game/UI/WBP_MainInterface.WBP_MainInterface_C|GetInteractionText (Variables|/Game/Characters/Player/Blueprints/BP_PlayerCharacter.BP_PlayerCharacter_C|GetMainUI _asbp_player_character)) "YOU CAN'T LEAVE WITHOUT THE GEMSTONE!"))))

(fn ConstructionScript)