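; Enemy AI controller that runs the BT_Enemy behavior tree and feeds AI Perception results into its Blackboard.
; Sight of the player character sets PlayerActor, and losing sight clears it and stores the stimulus location as LastKnownLocation.
; Hearing stimuli from any actor write their location to HearingLocation.
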(event OnTargetPerceptionUpdated(AIPerception)
  (params (Actor :type Actor%20Object%20Reference) (Stimulus :type AI%20Stimulus%20Structure))
  (CallFunction|HandleSight Actor Stimulus)
  (CallFunction|HandleHearing Actor Stimulus))

(event EventBeginPlay
  (AI|RunBehaviorTree "/Game/Characters/Enemies/BT_Enemy.BT_Enemy"))

(fn ConstructionScript)

(fn HandleSight
  (params (A :type Object%20Object%20Reference) (Stimulus :type AI%20Stimulus%20Structure%20%28by%20ref%29))
  (bind (_age _expirationage _strength _stimuluslocation _receiverlocation _tag _bsuccessfullysensed) (Utilities|Struct|BreakAIStimulus Stimulus))
  (bind _returnvalue (Class|AIPerceptionSystem|GetSenseClassforStimulus Stimulus))
  (if (and (== A (Game|GetPlayerCharacter 0)) (== _returnvalue "/Script/AIModule.AISense_Sight"))
    (AI|Components|Blackboard|SetValueasObject (Variables|Default|GetBlackboard) (Utilities|Name|MakeLiteralName "PlayerActor") (Utilities|SelectObject (Game|GetPlayerCharacter 0) 0 _bsuccessfullysensed))
    (if _bsuccessfullysensed
      (return)
      (else
        (AI|Components|Blackboard|SetValueasVector (Variables|Default|GetBlackboard) (Utilities|Name|MakeLiteralName "LastKnownLocation") _stimuluslocation)
        (return)))
    (else
      (return))))

(fn HandleHearing
  (params (Actor :type Actor%20Object%20Reference) (Stimulus :type AI%20Stimulus%20Structure))
  (bind _returnvalue (Class|AIPerceptionSystem|GetSenseClassforStimulus Stimulus))
  (if (== _returnvalue "/Script/AIModule.AISense_Hearing")
    (AI|Components|Blackboard|SetValueasVector (Variables|Default|GetBlackboard) (Utilities|Name|MakeLiteralName "HearingLocation") (.StimulusLocation (Utilities|Struct|BreakAIStimulus Stimulus)))))