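; Enemy character that deals contact damage to the player through a hit box while attacking is allowed, and takes five times damage when unaware.
; Non-lethal hits grant brief invulnerability.
; Death clears the blackboard's IsAlive key, hides the spotlight, stops movement and plays a death animation.
; UpdateState sets awareness and picks chase speed, or alert or patrol speed from the game instance's castle-alert flag.
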(event OnComponentBeginOverlap(HitBox)
  (params (OverlappedComponent :type Primitive%20Component%20Object%20Reference) (OtherActor :type Actor%20Object%20Reference) (OtherComp :type Primitive%20Component%20Object%20Reference) (OtherBodyIndex :type Integer) (bFromSweep :type Boolean) (SweepResult :type Hit%20Result%20Structure%20%28by%20ref%29))
  (if (and (Actor|ActorHasTag OtherActor "Player") (Variables|Default|GetB_CanAttack))
    (Game|Damage|ApplyDamage OtherActor 1e+01 0 0)))

(event Game|Damage|EventAnyDamage
  (params (Damage :type Float%20%28single-precision%29) (DamageType :type Damage%20Type%20Object%20Reference) (InstigatedBy :type Controller%20Object%20Reference) (DamageCauser :type Actor%20Object%20Reference))
  (bind _output_get (Variables|Default|SetHP (- (Variables|Default|GetHP) (* Damage (Math|Float|SelectFloat 1.0 5.0 (Variables|Default|GetB_IsAware))))))
  (Audio|PlaySoundatLocation "/Game/Audio/Effects/SC_ManDamage.SC_ManDamage" (Transformation|GetActorLocation) "0, 0, 0" 1.0 1.0 0.0 0 0 0 0)
  (if (<= _output_get 0.0)
    (Utilities|FlowControl|Sequence
      (:then_0
        (AI|Components|Blackboard|ClearValue (Variables|/Script/AIModule.AIController|GetBlackboard (AI|GetAIController self)) (Utilities|Name|MakeLiteralName "IsAlive"))
        (Rendering|SetVisibility (Variables|Default|GetSpotLight) false false))
      (:then_1
        (Components|Movement|StopMovementImmediately (Variables|Character|GetCharacterMovement))
        (Components|Animation|PlayAnimation (Variables|Character|GetMesh) "/Game/Characters/Animations/NewAL_StandardRig_Death01.NewAL_StandardRig_Death01" false)
        (Variables|Actor|SetbCanBeDamaged false)))
    (else
      (Variables|Actor|SetbCanBeDamaged false)
      (Utilities|FlowControl|Delay 0.5)
      (Variables|Actor|SetbCanBeDamaged true))))

(fn ConstructionScript)

(fn UpdateState
  (params (B_IsAware :type Boolean))
  (Variables|Default|SetB_IsAware B_IsAware)
  (CallFunction|UpdateMovementSpeed))

(fn UpdateMovementSpeed
  (if (Variables|Default|GetB_IsAware)
    (Variables|/Script/Engine.CharacterMovementComponent|SetMaxWalkSpeed (Variables|Character|GetCharacterMovement) (Variables|Default|GetChaseWalkSpeed))
    (else
      (bind _asbp_my_game_instance (Utilities|Casting|CastToBP_MyGameInstance (Game|GetGameInstance)))
      (if (Variables|/Game/Framework/Core/BP_MyGameInstance.BP_MyGameInstance_C|Getb_CastleAlerted _asbp_my_game_instance)
        (Variables|/Script/Engine.CharacterMovementComponent|SetMaxWalkSpeed (Variables|Character|GetCharacterMovement) (Variables|Default|GetAlertWalkSpeed))
        (else
          (Variables|/Script/Engine.CharacterMovementComponent|SetMaxWalkSpeed (Variables|Character|GetCharacterMovement) (Variables|Default|GetPatrolWalkSpeed)))))))